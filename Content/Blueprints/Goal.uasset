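; Goal actor that detects objects passing through it, using a sphere trigger and a mesh both sized from a Radius variable.
; On begin overlap it stores each component's entry position, unrotated into the goal's local space, in a map and draws a debug point.
; On end overlap it fires GOAL if local X changed sign, then removes the entry.
; GOAL currently only prints a message.
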(event OnComponentBeginOverlap(Sphere)
  (params (OverlappedComponent :type Primitive%20Component%20Object%20Reference) (OtherActor :type Actor%20Object%20Reference) (OtherComp :type Primitive%20Component%20Object%20Reference) (OtherBodyIndex :type Integer) (bFromSweep :type Boolean) (SweepResult :type Hit%20Result%20Structure%20%28by%20ref%29))
  (bind _returnvalue (Transformation|GetWorldLocation OtherComp))
  (bind _returnvalue_2 (Transformation|GetActorLocation))
  (bind _returnvalue_3 (Transformation|GetActorRotation))
  (bind _returnvalue_4 (- _returnvalue _returnvalue_2))
  (bind _returnvalue_5 (Math|Vector|UnrotateVector _returnvalue_4 _returnvalue_3))
  (Variables|Default|SetStartLoc _returnvalue_5)
  (Rendering|Debug|DrawDebugPoint (+ _returnvalue_4 _returnvalue_2) 25.0 "(R=0.091340,G=1.000000,B=0.000000,A=1.000000)" 2.0)
  (Utilities|Map|Add (Variables|Default|GetLocations) OtherComp _returnvalue_5))

(event OnComponentEndOverlap(Sphere)
  (params (OverlappedComponent :type Primitive%20Component%20Object%20Reference) (OtherActor :type Actor%20Object%20Reference) (OtherComp :type Primitive%20Component%20Object%20Reference) (OtherBodyIndex :type Integer))
  (bind _returnvalue (Transformation|GetActorLocation))
  (bind _returnvalue_2 (Transformation|GetActorRotation))
  (bind _returnvalue_3 (Transformation|GetWorldLocation OtherComp))
  (bind _locations (Variables|Default|GetLocations))
  (bind _returnvalue_4 (- _returnvalue_3 _returnvalue))
  (bind (_value _returnvalue_5) (Utilities|Map|Find _locations OtherComp))
  (bind _returnvalue_6 (Math|Vector|UnrotateVector _returnvalue_4 _returnvalue_2))
  (bind _x (Math|Vector|BreakVector _value))
  (bind _x_2 (Math|Vector|BreakVector _returnvalue_6))
  ;[1 1 1] on exit
  (if _returnvalue_5
    (Utilities|FlowControl|Sequence
      (:then_0
        (if (or (and (> _x_2 0.0) (< _x 0.0)) (and (< _x_2 0.0) (> _x 0.0)))
          (CallFunction|GOAL _value _returnvalue_6)
          (else
            (Development|PrintString "there has been a mistake here i think"))))
      (:then_1
        (Utilities|Map|Remove (Variables|Default|GetLocations) OtherComp)))
    (else
      (Development|PrintString "dude wtf how"))))

(event Custom|GOAL
  (params (Start :type Vector) (End :type Vector))
  ;[1 1 1] glao
  (Development|PrintString "GOAL"))

(event EventBeginPlay)

(event Collision|EventActorBeginOverlap
  (params (OtherActor :type Actor%20Object%20Reference)))

(event EventTick
  (params (DeltaSeconds :type Float%20%28single-precision%29)))

(fn ConstructionScript
  (bind _radius (Variables|Default|GetRadius))
  (bind _returnvalue (* _radius 0.0033))
  (Components|Sphere|SetSphereRadius (Variables|Default|GetSphere) _radius true)
  (Transformation|SetRelativeScale3D (Variables|Default|GetStaticMesh) (Math|Vector|MakeVector _returnvalue _returnvalue _returnvalue)))