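; Player character for a physics ball game, with wall running, dashing, crouching, ball kicking and lobbing, and switchable first/third-person cameras.
; While falling, Tick traces for walls, ignoring Ball_BP, and relaunches the character along the surface with curve-driven vertical speed and zero gravity.
; Holding Fire charges kick strength along a curve through a breakable delay-loop macro; release kicks.
; Kick, dash and lob share a sphere trace to push physics bodies.
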(event OnComponentBeginOverlap(Capsule)
  (params (OverlappedComponent :type Primitive%20Component%20Object%20Reference) (OtherActor :type Actor%20Object%20Reference) (OtherComp :type Primitive%20Component%20Object%20Reference) (OtherBodyIndex :type Integer) (bFromSweep :type Boolean) (SweepResult :type Hit%20Result%20Structure%20%28by%20ref%29))
  (Variables|Default|SetKickStart (- (Transformation|GetActorLocation) (Transformation|GetActorLocation OtherActor)))
  (Rendering|Debug|DrawDebugPoint :Size 25.0 :Duration 1.0)
  (Utilities|Time|SetTimerbyEvent (delegate Custom|CheckBallDistance) 0.01 true))

(event OnComponentEndOverlap(Capsule)
  (params (OverlappedComponent :type Primitive%20Component%20Object%20Reference) (OtherActor :type Actor%20Object%20Reference) (OtherComp :type Primitive%20Component%20Object%20Reference) (OtherBodyIndex :type Integer))
  (Utilities|Time|SetTimerbyEvent (delegate Custom|CheckBallDistance) 0.0))

(event Custom|KickBall
  (bind _returnvalue (Transformation|GetVelocity))
  (bind _returnvalue_2 (Pawn|GetControlRotation :!class /Script/Engine.Pawn))
  (bind _returnvalue_3 (Pawn|GetControlRotation :!class /Script/Engine.Pawn))
  (bind _returnvalue_4 (Math|Vector|GetForwardVector _returnvalue_2))
  (bind _returnvalue_5 (Math|Vector|GetForwardVector _returnvalue_3))
  (bind _returnvalue_6 (Math|Vector|DotProduct _returnvalue _returnvalue_4))
  (bind _returnvalue_7 (Math|Float|Clamp(Float) _returnvalue_6 0.0 1e+06))
  ;[1 1 1] kick ball
  (Variables|Default|SetJustKicked true)
  (Utilities|FlowControl|Sequence
    (:then_0
      (bind (_outhits _returnvalue_8) (CallFunction|BallTrace2 -1e+02 1e+02 1e+02 0.25))
      (if _returnvalue_8
        (for _array_element _outhits
          (Physics|AddImpulse (.HitComponent (Collision|BreakHitResult _array_element)) (* (Math|Vector|Normalize (Math|Vector|MakeVector (.x (Math|Vector|Lerp(Vector) (Math|Vector|Normalize (- (.ImpactPoint (Collision|BreakHitResult _array_element)) (.TraceStart (Collision|BreakHitResult _array_element)))) _returnvalue_5 0.75)) (.y (Math|Vector|Lerp(Vector) (Math|Vector|Normalize (- (.ImpactPoint (Collision|BreakHitResult _array_element)) (.TraceStart (Collision|BreakHitResult _array_element)))) _returnvalue_5 0.75)) (.Z (Math|Vector|BreakVector _returnvalue_5)))) (Math|Float|Lerp (+ (* _returnvalue_7 0.5) 7e+02) (+ (* _returnvalue_7 1e+01) 1.5e+04) (stale Input|ActionEvents|InputActionFire _output))) (.HitBoneName (Collision|BreakHitResult _array_element)) true))))
    (:then_1
      (Utilities|FlowControl|Delay 0.1)
      (Variables|Default|SetJustKicked false))))

(event Custom|CheckBallDistance)

(event Custom|StopWallRunning
  ;[1 1 1] wallrunniong
  (CallFunction|ResetMovementMode)
  (Utilities|FlowControl|DoOnce false) ; enters at Reset
)

(event Custom|Dash
  (bind _dashvelocity (Variables|Default|GetDashVelocity))
  (bind _dashvelocity_2 (Variables|Default|GetDashVelocity))
  (bind (_x _y) (Math|Vector2D|BreakVector2D _dashvelocity))
  ;[1 1 1] dash
  (if (Variables|Default|GetCanDash)
    (Variables|Default|SetCanDash false)
    (Character|LaunchCharacter (+ (* (Math|Vector|RotateVector (Variables|Default|GetMovementInput) (Transformation|GetActorRotation)) _x) (Math|Vector|MakeVector 0.0 0.0 _y)) false false)
    (bind (_outhits _returnvalue) (CallFunction|BallTrace2 -1e+02 1e+02 1e+02 0.25))
    (if _returnvalue
      (for _array_element _outhits
        (Class|PrimitiveComponent|SetAllPhysicsAngularVelocityinRadians (.HitComponent (Collision|BreakHitResult _array_element)) (Math|Vector|MakeVector 0.0 0.0 0.0) false)
        (Class|PrimitiveComponent|SetAllPhysicsLinearVelocity (.HitComponent (Collision|BreakHitResult _array_element)) (+ (Math|Vector|MakeVector (* (.x (Transformation|GetComponentVelocity (.HitComponent (Collision|BreakHitResult _array_element)))) (Math|Float|MapRangeClamped (Math|Vector|VectorLength (- (.TraceStart (Collision|BreakHitResult _array_element)) (.ImpactPoint (Collision|BreakHitResult _array_element)))) 0.0 2e+02 0.15 1.0)) (* (.y (Transformation|GetComponentVelocity (.HitComponent (Collision|BreakHitResult _array_element)))) (Math|Float|MapRangeClamped (Math|Vector|VectorLength (- (.TraceStart (Collision|BreakHitResult _array_element)) (.ImpactPoint (Collision|BreakHitResult _array_element)))) 0.0 2e+02 0.15 1.0)) (* (.z (Transformation|GetComponentVelocity (.HitComponent (Collision|BreakHitResult _array_element)))) 0.5)) (* (Math|Vector|RotateVector (Variables|Default|GetMovementInput) (Transformation|GetActorRotation)) (* (.x _dashvelocity_2) 2.5)) (Math|Vector|MakeVector 0.0 0.0 (* (.y _dashvelocity_2) 1.5)) (* (Transformation|GetVelocity) 0.5)) false)))))

(event EventTick
  (params (DeltaSeconds :type Float%20%28single-precision%29))
  (bind _returnvalue (Transformation|GetVelocity))
  (bind _returnvalue_2 (Transformation|GetVelocity))
  (bind _returnvalue_3 (Transformation|GetActorLocation))
  (bind _charactermovement (Variables|Character|GetCharacterMovement))
  (bind (_x _y) (Math|Vector|BreakVector _returnvalue_2))
  ;[1 1 1] wallrunniong
  (Utilities|FlowControl|Sequence
    (:then_0
      (if (and (Variables|Default|GetCanWallRun) (AI|Components|NavMovement|IsFalling (Variables|Character|GetCharacterMovement)))
        (bind (_outhit _returnvalue_4) (CallFunction|WallTrace 1.5))
        (if _returnvalue_4
          (Utilities|FlowControl|Sequence
            (:then_0
              (Utilities|FlowControl|DoOnce false :!label _label
                (:Completed
                  (Variables|Default|SetWallRunVelocity (Transformation|GetVelocity))
                  (Variables|Default|SetCanDash true)
                  (Variables|Default|SetWallTime 0.0))))
            (:then_1
              (Variables|Default|SetWallRunning true)
              (Rendering|Debug|DrawDebugArrow _returnvalue_3 (+ _returnvalue_3 (* (Math|Vector|Normalize (CallFunction|ConverttoWallVelocity (.Normal (Collision|BreakHitResult _outhit)) (Math|Interpolation|VInterpTo _returnvalue_2 (Math|Vector|MakeVector _x _y (+ (Math|Curves|GetFloatValue (Variables|Default|GetWallCurve) (Variables|Default|GetWallTime)) (* (Math|Float|Clamp(Float) (Math|Vector|DotProduct (.Normal (Collision|BreakHitResult _outhit)) (* (Math|Vector|RotateVector (Variables|Default|GetMovementInput) (Transformation|GetActorRotation)) -1.0))) 5e+02))) (Utilities|Time|GetWorldDeltaSeconds) 1.0))) 1e+02)) 1e+01 "(R=0.000000,G=0.048569,B=0.822917,A=1.000000)" 0.0 2.0)
              (Variables|/Script/Engine.CharacterMovementComponent|SetGravityScale _charactermovement 0.0)
              (Variables|/Script/Engine.CharacterMovementComponent|SetAirControl _charactermovement (Math|Float|MapRangeClamped (Math|Vector|VectorLength (Math|Vector|MakeVector (.x _returnvalue) (.y _returnvalue) 0.0)) 1e+02 3e+02 0.0 1.0))
              (Variables|/Script/Engine.CharacterMovementComponent|SetFallingLateralFriction _charactermovement 0.5)
              (Character|LaunchCharacter (CallFunction|ConverttoWallVelocity (.Normal (Collision|BreakHitResult _outhit)) (Math|Interpolation|VInterpTo _returnvalue_2 (Math|Vector|MakeVector _x _y (+ (Math|Curves|GetFloatValue (Variables|Default|GetWallCurve) (Variables|Default|GetWallTime)) (* (Math|Float|Clamp(Float) (Math|Vector|DotProduct (.Normal (Collision|BreakHitResult _outhit)) (* (Math|Vector|RotateVector (Variables|Default|GetMovementInput) (Transformation|GetActorRotation)) -1.0))) 5e+02))) (Utilities|Time|GetWorldDeltaSeconds) 1.0)) true true)
              (bind _output_get (Variables|Default|SetWallTime (+ (stale _output_get) (Utilities|Time|GetWorldDeltaSeconds))))
              (Development|PrintString (Utilities|String|ToString(Float) _output_get))))
          (else
            (CallFunction|ResetMovementMode)
            (goto _label Reset)))
        (else
          (CallFunction|ResetMovementMode))))
    (:then_1
      (Transformation|SetRelativeLocation (Variables|Default|GetFPcamera) (Math|Vector|MakeVector (* (Math|Vector|DotProduct (Math|Vector|GetForwardVector (Pawn|GetControlRotation :!class /Script/Engine.Pawn)) "0, 0,1.000000") -2e+01) 0.0 (.z (Variables|/Script/Engine.SceneComponent|GetRelativeLocation (Variables|Default|GetFPcamera)))) false false))))

(event EventOnLanded
  (params (Hit :type Hit%20Result%20Structure%20%28by%20ref%29))
  (CallFunction|StopWallRunning)
  (Variables|Default|SetCanWallRun true)
  (Variables|Default|SetCanLob true)
  (Variables|Default|SetCanDash true)
  (Utilities|FlowControl|Delay 0.2)
  (Variables|Default|SetJustDashed false))

(event Input|ActionEvents|InputActionCrouchHold
  (params (Key :type Key%20Structure))
  (:Pressed
    (Character|Crouch))
  (:Released
    (Character|UnCrouch)))

(event Input|ActionEvents|InputActionDash
  (params (Key :type Key%20Structure))
  (:Pressed
    (CallFunction|Dash)))

(event Input|ActionEvents|InputActionJump
  (params (Key :type Key%20Structure))
  (bind _returnvalue (Transformation|GetVelocity))
  (:Pressed
    (if (and (Variables|Default|GetJustDashed) (Pawn|Components|CharacterMovement|IsWalking (Variables|Character|GetCharacterMovement)))
      (Character|LaunchCharacter (Math|Vector|MakeVector (.x _returnvalue) (.y _returnvalue) (Variables|/Script/Engine.CharacterMovementComponent|GetJumpZVelocity (Variables|Character|GetCharacterMovement))) false false)
      (Variables|Default|SetJustDashed false)
      (else
        (Character|Jump)
        (if (Variables|Default|GetWallRunning)
          (CallFunction|Dash)
          (Variables|Default|SetCanWallRun false)
          (Utilities|FlowControl|Delay 0.5)
          (Variables|Default|SetCanWallRun true))))))

(event Input|ActionEvents|InputActionFire
  (params (Key :type Key%20Structure))
  ;[1 1 1] kick ball
  (:Pressed
    (bind (_output _stepsize) (Utilities|MdelayCurve 0.0 1.0 0.01 true "/Game/Blueprints/KickStrengthCurve.KickStrengthCurve" :!label _label)
      (:then
        (Development|PrintString (Utilities|String|ToString(Float) _output) true true "(R=0.000000,G=0.660000,B=1.000000,A=1.000000)" _stepsize))
      (:onBreak
        (CallFunction|KickBall))))
  (:Released
    (goto _label Break)))

(event Input|ActionEvents|InputActionAim
  (params (Key :type Key%20Structure))
  ;[1 1 1] lob ball
  (:Pressed
    (if (Variables|Default|GetCanLob)
      (Variables|Default|SetCanLob false)
      (Utilities|FlowControl|Sequence
        (:then_0
          (bind (_outhits _returnvalue) (CallFunction|BallTrace2 -1e+02 1e+02 1e+02 0.25))
          (if _returnvalue
            (for _array_element _outhits
              (Class|PrimitiveComponent|SetAllPhysicsLinearVelocity (.HitComponent (Collision|BreakHitResult _array_element)) (+ (* (Transformation|GetVelocity) 0.5) (Math|Vector|MakeVector (.x (Transformation|GetComponentVelocity (.HitComponent (Collision|BreakHitResult _array_element)))) (.y (Transformation|GetComponentVelocity (.HitComponent (Collision|BreakHitResult _array_element)))) (* (.z (Transformation|GetComponentVelocity (.HitComponent (Collision|BreakHitResult _array_element)))) 0.5)) "0,0,750.000000") false))))
        (:then_1
          (Utilities|FlowControl|Delay 0.25)
          (Variables|Default|SetCanLob true))))))

(event Input|AxisEvents|InputAxisMoveRight
  (params (AxisValue :type Float%20%28single-precision%29))
  ;[1 1 1] Comment
  (Pawn|Input|AddMovementInput (.Y (Math|Rotator|GetAxes (Math|Rotator|MakeRotator 0.0 0.0 (.yaw (Pawn|GetControlRotation :!class /Script/Engine.Pawn))))) AxisValue false)
  (bind _output_get (Variables|Default|SetMovementInput (Math|Vector|MakeVector (stale Input|AxisEvents|InputAxisMoveForward AxisValue) AxisValue 0.0)))
  (Variables|Default|SetMovementInput (Math|Vector|Normalize _output_get)))

(event Input|AxisEvents|InputAxisMoveForward
  (params (AxisValue :type Float%20%28single-precision%29))
  ;[1 1 1] Comment
  (Pawn|Input|AddMovementInput (.X (Math|Rotator|GetAxes (Math|Rotator|MakeRotator 0.0 0.0 (.yaw (Pawn|GetControlRotation :!class /Script/Engine.Pawn))))) AxisValue false)
  (bind _output_get (Variables|Default|SetMovementInput (Math|Vector|MakeVector AxisValue (stale Input|AxisEvents|InputAxisMoveRight AxisValue) 0.0)))
  (Variables|Default|SetMovementInput (Math|Vector|Normalize _output_get)))

(event Input|AxisEvents|InputAxisLookRight
  (params (AxisValue :type Float%20%28single-precision%29))
  ;[1 1 1] Comment
  (Pawn|Input|AddControllerYawInput AxisValue))

(event Input|AxisEvents|InputAxisLookUp
  (params (AxisValue :type Float%20%28single-precision%29))
  ;[1 1 1] Comment
  (Pawn|Input|AddControllerPitchInput AxisValue))

(event Input|KeyboardEvents|V
  (params (Key :type Key%20Structure))
  (bind _tpcamera (Variables|Default|GetTPcamera))
  (bind _returnvalue (Components|Activation|IsActive _tpcamera))
  (:Pressed
    (Components|Activation|SetActive (Variables|Default|GetFPcamera) _returnvalue false)
    (Components|Activation|SetActive _tpcamera (not _returnvalue) false)))

(fn ConstructionScript
  (bind _capsulecomponent (Variables|Collision|GetCapsuleComponent))
  (bind _capsule (Variables|Default|GetCapsule))
  (bind _capsulecomponent_2 (Variables|Collision|GetCapsuleComponent))
  (Transformation|SetRelativeLocation (Variables|Default|GetFPcamera) (Math|Vector|MakeVector 0.0 0.0 (- (Variables|/Script/Engine.CapsuleComponent|GetCapsuleHalfHeight _capsulecomponent) (Variables|/Script/Engine.CapsuleComponent|GetCapsuleRadius _capsulecomponent))) false false)
  (Components|Capsule|SetCapsuleHalfHeight _capsule (Variables|/Script/Engine.CapsuleComponent|GetCapsuleHalfHeight _capsulecomponent_2) true)
  (Components|Capsule|SetCapsuleRadius _capsule (Variables|/Script/Engine.CapsuleComponent|GetCapsuleRadius _capsulecomponent_2) true))

(fn KickBallTraceFunction
  (params (Direction :type Vector) (DirectionMultiplier :type Float%20%28single-precision%29) (Plus :type Vector) (ForwardIf0 :type Boolean))
  (bind _returnvalue (Transformation|GetActorLocation))
  (bind _returnvalue_2 (Transformation|GetActorUpVector))
  (bind _capsulecomponent (Variables|Collision|GetCapsuleComponent))
  (bind _kickcapsuleradius (Variables|Default|GetKickCapsuleRadius))
  (bind _capsulehalfheight (Variables|/Script/Engine.CapsuleComponent|GetCapsuleHalfHeight _capsulecomponent))
  (bind _returnvalue_3 (- _capsulehalfheight _kickcapsuleradius))
  (bind _returnvalue_4 (* _returnvalue_2 _returnvalue_3))
  (bind _returnvalue_5 (- _returnvalue _returnvalue_4))
  (bind (_outhits _returnvalue_6) (Collision|MultiSphereTraceForObjects _returnvalue_5 (+ _returnvalue_5 (* (Transformation|GetActorForwardVector) 1.5e+02)) (Variables|Default|GetKickCapsuleRadius) (Utilities|Array|MakeArray "ObjectTypeQuery4") false 0 "ForDuration"))
  (if _returnvalue_6
    (Physics|AddImpulse (.HitComponent (Collision|BreakHitResult (Utilities|Array|Get(acopy) _outhits))) (+ (* (select (and ForwardIf0 (Math|Vector|Equal(Vector) Direction "0, 0, 0" 0.0001)) (Transformation|GetActorForwardVector) Direction) DirectionMultiplier) Plus) "None" false)))

(fn BallTrace
  (params (Direction :type Vector) (Length :type Float%20%28single-precision%29) (DrawDebugType :type EDrawDebugTrace%20Enum :default "ForDuration"))
  (bind _returnvalue (Transformation|GetActorForwardVector))
  (bind _returnvalue_2 (Transformation|GetActorLocation))
  (bind _returnvalue_3 (Transformation|GetActorUpVector))
  (bind _capsulecomponent (Variables|Collision|GetCapsuleComponent))
  (bind _kickcapsuleradius (Variables|Default|GetKickCapsuleRadius))
  (bind _returnvalue_4 (* _returnvalue _kickcapsuleradius))
  (bind _returnvalue_5 (* _kickcapsuleradius 0.5))
  (bind _capsulehalfheight (Variables|/Script/Engine.CapsuleComponent|GetCapsuleHalfHeight _capsulecomponent))
  (bind _returnvalue_6 (* _returnvalue_4 0.5))
  (bind _returnvalue_7 (- _capsulehalfheight _returnvalue_5))
  (bind _returnvalue_8 (* _returnvalue_3 _returnvalue_7))
  (bind _returnvalue_9 (+ _returnvalue_2 _returnvalue_6))
  (bind _returnvalue_10 (- _returnvalue_9 _returnvalue_8))
  (bind (_outhits _returnvalue_11) (Collision|MultiSphereTraceForObjects (- _returnvalue_10 (* (Transformation|GetActorForwardVector) 1e+02)) (+ _returnvalue_10 (* Direction Length)) (Variables|Default|GetKickCapsuleRadius) (Utilities|Array|MakeArray "ObjectTypeQuery4") false 0 DrawDebugType))
  (return _returnvalue_11 (Utilities|Array|Get(acopy) _outhits)))

(fn ResetMovementMode
  (bind _charactermovement (Variables|Character|GetCharacterMovement))
  (Variables|Default|SetWallRunning false)
  (Variables|/Script/Engine.CharacterMovementComponent|SetFallingLateralFriction _charactermovement 0.0)
  (Variables|/Script/Engine.CharacterMovementComponent|SetAirControl _charactermovement 0.25)
  (Variables|/Script/Engine.CharacterMovementComponent|SetGravityScale _charactermovement 1.0)
  (Pawn|Components|CharacterMovement|SetMovementMode (Variables|Character|GetCharacterMovement) (select (AI|Components|NavMovement|IsFalling _charactermovement) "MOVE_Falling" "MOVE_Walking") 0))

(fn WallTrace
  (params (RadiusMultiplier :type Float%20%28single-precision%29))
  (bind _returnvalue (Transformation|GetVelocity))
  (bind _returnvalue_2 (Transformation|GetActorLocation))
  (bind _returnvalue_3 (Transformation|GetActorUpVector))
  (bind _returnvalue_4 (Transformation|GetActorLocation))
  (bind _capsulecomponent (Variables|Collision|GetCapsuleComponent))
  (bind _capsulecomponent_2 (Variables|Collision|GetCapsuleComponent))
  (bind _capsulehalfheight (Variables|/Script/Engine.CapsuleComponent|GetCapsuleHalfHeight _capsulecomponent))
  (bind _capsuleradius (Variables|/Script/Engine.CapsuleComponent|GetCapsuleRadius _capsulecomponent_2))
  (bind _returnvalue_5 (* _capsuleradius RadiusMultiplier))
  (bind _returnvalue_6 (* _returnvalue_5 1.1))
  (bind _returnvalue_7 (- _capsulehalfheight _returnvalue_6))
  (bind _returnvalue_8 (* _returnvalue_3 _returnvalue_7))
  (bind (_outhit _returnvalue_9) (Collision|SphereTraceByChannel (- _returnvalue_2 _returnvalue_8) (+ _returnvalue_2 _returnvalue_8) _returnvalue_5 "TraceTypeQuery1" false 0 "ForOneFrame"))
  (if _returnvalue_9
    (bind (_outhit_2 _returnvalue_10) (Collision|LineTraceByChannel _returnvalue_4 (- _returnvalue_4 (- (* (.Normal (Collision|BreakHitResult _outhit)) (* (Variables|/Script/Engine.CapsuleComponent|GetCapsuleRadius (Variables|Collision|GetCapsuleComponent)) RadiusMultiplier)) (* (Math|Vector|Normalize (Math|Vector|MakeVector (.x _returnvalue) (.y _returnvalue) (.z _returnvalue))) 1e+01))) "TraceTypeQuery1" false 0 "ForOneFrame"))
    (Utilities|Casting|CastToBall_BP (.HitActor (Collision|BreakHitResult _outhit_2))
      (:then
        (return "" false))
      (:CastFailed
        (return _outhit_2 _returnvalue_10)))
    (else
      (return "" false))))

(fn ConverttoWallVelocity
  (params (Normal :type Vector%20%28by%20ref%29) (Velocity :type Vector))
  (bind _returnvalue (* Normal -0.1))
  (bind _returnvalue_2 (Math|Vector|Normalize Velocity))
  (bind _returnvalue_3 (Math|Rotator|MakeRotfromZX Normal _returnvalue_2))
  (bind _returnvalue_4 (Math|Vector|GetForwardVector _returnvalue_3))
  (bind _returnvalue_5 (+ _returnvalue_4 _returnvalue))
  (return (* _returnvalue_5 (Math|Vector|DotProduct _returnvalue_5 Velocity))))

(fn BallTrace2
  (params (Start :type Float%20%28single-precision%29) (End :type Float%20%28single-precision%29) (Radius :type Float%20%28single-precision%29) (Feet%20/%20Head :type Float%20%28single-precision%29))
  (bind _returnvalue (Transformation|GetActorForwardVector))
  (bind _returnvalue_2 (Transformation|GetActorLocation))
  (bind _returnvalue_3 (Transformation|GetActorUpVector))
  (bind _capsulecomponent (Variables|Collision|GetCapsuleComponent))
  (bind _returnvalue_4 (* _returnvalue Radius))
  (bind _capsulehalfheight (Variables|/Script/Engine.CapsuleComponent|GetCapsuleHalfHeight _capsulecomponent))
  (bind _returnvalue_5 (* _returnvalue_4 0.5))
  (bind _returnvalue_6 (* _capsulehalfheight -1.0))
  (bind _returnvalue_7 (Math|Float|Lerp _capsulehalfheight _returnvalue_6 Feet%20/%20Head))
  (bind _returnvalue_8 (+ _returnvalue_2 _returnvalue_5))
  (bind _returnvalue_9 (* _returnvalue_3 _returnvalue_7))
  (bind _returnvalue_10 (- _returnvalue_8 _returnvalue_9))
  (bind (_outhits _returnvalue_11) (Collision|MultiSphereTraceForObjects (+ (* (Transformation|GetActorForwardVector) Start) _returnvalue_10) (+ _returnvalue_10 (* (Math|Vector|GetForwardVector (Pawn|GetControlRotation :!class /Script/Engine.Pawn)) End)) Radius (Utilities|Array|MakeArray "ObjectTypeQuery4") false 0 "ForDuration"))
  (return _outhits _returnvalue_11))