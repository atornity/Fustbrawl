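; Ball spawner actor that launches Ball_BP actors at a set velocity from its Cube marker.
; Tick drives delayed spawning when the Capsule overlaps nothing, capping the ball count and culling balls beyond a maximum distance.
; The construction script traces down to stretch the Capsule to the surface below, places the Cube along that span and previews the predicted trajectory with arrows.
; A scale-interpolation branch for the newest ball is unconnected.
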(event Custom|SpawnBall
  (bind _balls (Variables|Default|GetBalls))
  (bind _balls_2 (Variables|Default|GetBalls))
  (bind _output (Utilities|Array|Get(acopy) _balls_2))
  (if (< (Utilities|Array|Length (Class|PrimitiveComponent|GetOverlappingComponents (Variables|Default|GetCapsule))) 1)
    (Utilities|FlowControl|Delay (Variables|Default|GetTimer))
    (bind _returnvalue (Game|SpawnActorfromClass "/Game/Blueprints/Ball_BP.Ball_BP_C" (Math|Transform|MakeTransform (Transformation|GetWorldLocation (Variables|Default|GetCube)) "0, 0, 0" "1,1,1") "Undefined" 0 0))
    (Variables|/Game/Blueprints/Ball_BP.Ball_BP_C|SetRadius _returnvalue 4e+01)
    (Class|PrimitiveComponent|SetAllPhysicsLinearVelocity (Variables|/Game/Blueprints/Ball_BP.Ball_BP_C|GetBallMesh _returnvalue) (Variables|Default|GetVelocity) false)
    (Utilities|Array|Add _balls _returnvalue)
    (if (> (Utilities|Array|Length _balls) (Variables|Default|GetMaxBalls))
      (Actor|DestroyActor _output)
      (Utilities|Array|RemoveItem (Variables|Default|GetBalls) _output))))

(event Custom|BallsCleanup
  (Utilities|FlowControl|Delay 1.0)
  (for _array_element (Variables|Default|GetBalls)
    (if (> (Math|Vector|VectorLength (- (Transformation|GetActorLocation _array_element) (Transformation|GetActorLocation))) (Variables|Default|GetMaxDistance))
      (Actor|DestroyActor _array_element)
      (Utilities|Array|RemoveItem (Variables|Default|GetBalls) _array_element))))

(event EventTick
  (params (DeltaSeconds :type Float%20%28single-precision%29))
  (CallFunction|SpawnBall)
  (CallFunction|BallsCleanup))

(fn ConstructionScript
  (bind _returnvalue (Transformation|GetActorLocation))
  (bind _capsule (Variables|Default|GetCapsule))
  (bind (_outhit _returnvalue_2) (Collision|LineTraceByChannel _returnvalue (- _returnvalue "0, 0,10000000.000000") "TraceTypeQuery1" false 0 "None"))
  (if _returnvalue_2
    (Components|Capsule|SetCapsuleHalfHeight _capsule (Math|Vector|VectorLength (* (- (.ImpactPoint (Collision|BreakHitResult _outhit)) (.TraceStart (Collision|BreakHitResult _outhit))) 0.5)) true)
    (Transformation|SetRelativeLocation _capsule (* (- (.ImpactPoint (Collision|BreakHitResult _outhit)) (.TraceStart (Collision|BreakHitResult _outhit))) 0.5) false false)
    (Transformation|SetRelativeLocation (Variables|Default|GetCube) (Math|Vector|Lerp(Vector) (+ (- (.ImpactPoint (Collision|BreakHitResult _outhit)) (.TraceStart (Collision|BreakHitResult _outhit))) (Math|Vector|MakeVector 0.0 0.0 5e+01)) "0, 0, 0" (Variables|Default|GetspawnLocation)) false false)
    (bind _outpathpositions (Class|GameplayStatics|BlueprintPredictProjectilePathbyTraceChannel (Transformation|GetActorLocation) (Variables|Default|GetVelocity) true 0.0 "ECC_WorldDynamic" false 0 "ForDuration"))
    (for (_array_element _array_index) _outpathpositions
      (if (> _array_index 0)
        (AddComponent|AddArrowComponent true (Math|Transform|MakeTransform _array_element (Math|Conversions|RotationFromXVector (- _array_element (Utilities|Array|Get(acopy) _outpathpositions (- _array_index 1)))) "1,1,1"))))))